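; BP_Skeleton5 is an enemy skeleton that chases and attacks the player.
; Tick drives AI MoveTo until within reach, then plays an attack montage and rechecks distance to the player controller.
; Overlaps on the attack collision, disabled at BeginPlay, damage BP_AdventureMan, throttled by a delayed DoOnce reset.
; AnyDamage reduces health; at zero it notifies BP_GM_Metro, increments the player's kill count and destroys the actor after a short delay.
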(event OnComponentBeginOverlap(AttackingCollision)
  (params (OverlappedComponent :type Primitive%20Component%20Object%20Reference) (OtherActor :type Actor%20Object%20Reference) (OtherComp :type Primitive%20Component%20Object%20Reference) (OtherBodyIndex :type Integer) (bFromSweep :type Boolean) (SweepResult :type Hit%20Result%20Structure%20%28by%20ref%29))
  (bind _asbp_adventure_man (Utilities|Casting|CastToBP_AdventureMan OtherActor))
  (Utilities|FlowControl|DoOnce false
    (:Completed
      (Default|GetDamage _asbp_adventure_man (Variables|Default|GetSkeleton5Damage))
      (Utilities|FlowControl|Delay 1.0)
      (CallFunction|ResetAttackDoOnce))))

(event Custom|ResetAnimeAttack
  (Utilities|FlowControl|DoOnce false) ; enters at Reset
)

(event Custom|ResetAttackDoOnce
  (Utilities|FlowControl|DoOnce false) ; enters at Reset
)

(event Custom|Death
  (Utilities|IsValid 0))

(event Collision|EventActorBeginOverlap
  (params (OtherActor :type Actor%20Object%20Reference)))

(event EventBeginPlay
  (Collision|SetCollisionEnabled (Variables|Default|GetAttackingCollision) "NoCollision")
  (bind _asbp_gm_metro (Utilities|Casting|CastToBP_GM_Metro (Game|GetGameMode)))
  (Variables|Default|SetGMRef _asbp_gm_metro))

(event EventTick
  (params (DeltaSeconds :type Float%20%28single-precision%29))
  (if (not (Variables|Default|GetCanAttack?))
    (AI|AIMoveTo self "0, 0, 0" (Game|GetPlayerCharacter 0) (Variables|Default|GetCanReach?) true
      (:OnSuccess
        (Variables|Default|SetCanAttack? true)
        (Utilities|FlowControl|DoOnce false
          (:Completed
            (Animation|PlayAnimMontage "/Game/Mobs/Montages/Attack5_Montage.Attack5_Montage" 1.0 "None")
            (Utilities|FlowControl|Delay 1.0)
            (CallFunction|ResetAnimeAttack)
            (if (<= (Transformation|GetDistanceTo (Game|GetPlayerController 0)) (Variables|Default|GetCanReach?))
              (Variables|Default|SetCanAttack? true)
              (else
                (Variables|Default|SetCanAttack? false)))))))))

(event Game|Damage|EventAnyDamage
  (params (Damage :type Float%20%28single-precision%29) (DamageType :type Damage%20Type%20Object%20Reference) (InstigatedBy :type Controller%20Object%20Reference) (DamageCauser :type Actor%20Object%20Reference))
  (if (Variables|Default|GetIsAlive?)
    (bind _output_get (Variables|Default|SetHealth (- (Variables|Default|GetHealth) Damage)))
    (if (<= _output_get 0.0)
      (Variables|Default|SetIsAlive? false)
      (bind _asbp_gm_metro (Utilities|Casting|CastToBP_GM_Metro (Game|GetGameMode)))
      (bind _output_get_2 (Variables|Default|SetGMRef _asbp_gm_metro))
      (Utilities|FlowControl|DoOnce false
        (:Completed
          (Default|SkeletonDeath _output_get_2)
          (Utilities|FlowControl|Sequence
            (:then_0
              (bind _asbp_adventure_man (Utilities|Casting|CastToBP_AdventureMan (Game|GetPlayerCharacter 0)))
              (Math|Integer|IncrementInt (Variables|/Game/Blueprints/Player/BP_AdventureMan.BP_AdventureMan_C|GetCount_Kills _asbp_adventure_man)))
            (:then_1
              (Utilities|FlowControl|Delay 0.2)
              (Actor|DestroyActor))))))))

(fn ConstructionScript)