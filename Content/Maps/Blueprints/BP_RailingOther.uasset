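; BP_RailingOther is a metro railing obstacle that the player can remove by pressing E while nearby.
; A box overlap with BP_AdventureMan enables input and shows a BP_DoorCost widget with Game and UI input mode; leaving disables input and removes all widgets.
; E shrinks the mesh through chained scale steps and delays, then destroys the actor, with no cost check in this Blueprint.
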(event OnComponentBeginOverlap(Box)
  (params (OverlappedComponent :type Primitive%20Component%20Object%20Reference) (OtherActor :type Actor%20Object%20Reference) (OtherComp :type Primitive%20Component%20Object%20Reference) (OtherBodyIndex :type Integer) (bFromSweep :type Boolean) (SweepResult :type Hit%20Result%20Structure%20%28by%20ref%29))
  (Utilities|Casting|CastToBP_AdventureMan OtherActor)
  (Input|EnableInput (Game|GetPlayerController 0))
  (bind _returnvalue (UserInterface|CreateWidget "/Game/Maps/Blueprints/BP_DoorCost.BP_DoorCost_C"))
  (UserInterface|Viewport|AddtoViewport _returnvalue 0)
  (Input|SetInputModeGameandUI (Game|GetPlayerController 0) _returnvalue "DoNotLock" true false))

(event OnComponentEndOverlap(Box)
  (params (OverlappedComponent :type Primitive%20Component%20Object%20Reference) (OtherActor :type Actor%20Object%20Reference) (OtherComp :type Primitive%20Component%20Object%20Reference) (OtherBodyIndex :type Integer))
  (Utilities|Casting|CastToBP_AdventureMan OtherActor)
  (Input|DisableInput (Game|GetPlayerController 0))
  (Viewport|RemoveAllWidgets))

(event Input|KeyboardEvents|E
  (params (Key :type Key%20Structure))
  (:Pressed
    (Transformation|SetRelativeScale3D (Variables|Default|GetSM_Metro_railing_rb_1_b) "0.900000,0.900000,0.900000")
    (Utilities|FlowControl|Delay 0.1)
    (Transformation|SetRelativeScale3D (Variables|Default|GetSM_Metro_railing_rb_1_b) "0.800000,0.800000,0.800000")
    (Utilities|FlowControl|Delay 0.1)
    (Transformation|SetRelativeScale3D (Variables|Default|GetSM_Metro_railing_rb_1_b) "0.700000,0.700000,0.700000")
    (Utilities|FlowControl|Delay 0.1)
    (Transformation|SetRelativeScale3D (Variables|Default|GetSM_Metro_railing_rb_1_b) "0.600000,0.600000,0.600000")
    (Utilities|FlowControl|Delay 0.1)
    (Transformation|SetRelativeScale3D (Variables|Default|GetSM_Metro_railing_rb_1_b) "0.500000,0.500000,0.500000")
    (Utilities|FlowControl|Delay 0.1)
    (Transformation|SetRelativeScale3D (Variables|Default|GetSM_Metro_railing_rb_1_b) "0.400000,0.400000,0.400000")
    (Utilities|FlowControl|Delay 0.1)
    (Transformation|SetRelativeScale3D (Variables|Default|GetSM_Metro_railing_rb_1_b) "0.300000,0.300000,0.300000")
    (Utilities|FlowControl|Delay 0.1)
    (Transformation|SetRelativeScale3D (Variables|Default|GetSM_Metro_railing_rb_1_b) "0.200000,0.200000,0.200000")
    (Utilities|FlowControl|Delay 0.1)
    (Transformation|SetRelativeScale3D (Variables|Default|GetSM_Metro_railing_rb_1_b) "0.100000,0.100000,0.100000")
    (Utilities|FlowControl|Delay 0.1)
    (Actor|DestroyActor)))

(fn ConstructionScript)