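; Player character for a wave-based skeleton shooter, handling Enhanced Input movement, two-slot weapons, damage and game over.
; Weapons snap to hand or back sockets on pickup and swap, with camera line-trace gunfire, delay-looped auto fire, aim zoom and montage-based katana attacks.
; Money pays for obstacles and health, ammo or power-up vending machines.
; It creates and updates the HUD, pickup prompt, staged damage overlay, pause and end-game widgets.
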(event Custom|GetDamage
  (params (DamageTaken :type Float%20%28double-precision%29))
  ;[0.15 0.15 0.15 0.5] Get damage
  (bind _output_get (Variables|Default|SetHealth (- (Variables|Default|GetHealth) DamageTaken)))
  (Utilities|TakeDamageVisibility
    (:output
      (if (== (Variables|Default|GetHealth) 0.0)
        (Components|Animation|PlayAnimation (Variables|Character|GetMesh) "/Game/RifleAnimationAdventureMan/RifleAdventureManDeath_Ironsights_2.RifleAdventureManDeath_Ironsights_2" false)
        (bind _returnvalue (UserInterface|CreateWidget "/Game/Blueprints/UI/ENDGAME/WBP_EndGame.WBP_EndGame_C"))
        (Audio|PlaySound2D "/Game/Sound/GameOverMusic.GameOverMusic" 1.0 1.0 0.0 0 0)
        (UserInterface|Viewport|AddtoViewport _returnvalue 0)
        (Components|Movement|StopMovementImmediately (Variables|Character|GetCharacterMovement))
        (Input|DisableInput (Game|GetPlayerCharacter 0) (Game|GetPlayerController 0))
        (Variables|/Script/Engine.PlayerController|SetbShowMouseCursor (Game|GetPlayerController 0) true)
        (bind _asbp_gm_metro (Utilities|Casting|CastToBP_GM_Metro (Game|GetGameMode)))
        (Default|UpdateInfoGameOver _returnvalue (Variables|/Game/Blueprints/BP_GM_Metro.BP_GM_Metro_C|GetCurrent%20Wave _asbp_gm_metro) (Variables|/Game/Blueprints/BP_GM_Metro.BP_GM_Metro_C|GetTotalSkeletonKilled _asbp_gm_metro))))))

(event Custom|ContinueFire
  (bind _returnvalue (Game|GetPlayerCameraManager 0))
  (bind _hudref (Variables|Default|GetHUDRef))
  (bind _returnvalue_2 (Camera|GetCameraLocation _returnvalue))
  ;[0.15 0.15 0.15 0.5] Attack
  ;;[0.15 0.15 0.15 0.5] RifleAttack
  (bind _asbp_master_range (Utilities|Casting|CastToBP_MasterRange (Variables|Default|GetMain%20Weapon)))
  (if (> (Variables|/Game/Blueprints/Weapons/BP_MasterRange.BP_MasterRange_C|GetAmmo _asbp_master_range) 0)
    (bind _result (Math|Integer|DecrementInt (Variables|/Game/Blueprints/Weapons/BP_MasterRange.BP_MasterRange_C|GetAmmo _asbp_master_range))
      (:%20%20
        (switch Utilities|FlowControl|Switch|SwitchonEnum_WeaponNAME (Variables|/Game/Blueprints/Weapons/BP_MasterWeapons.BP_MasterWeapons_C|GetWeapon%20Name _asbp_master_range)
          (:NewEnumerator3
            (Default|UpdateAmmoNumber _hudref _result (Variables|Default|GetAssaultRifleAmmo)))
          (:NewEnumerator4
            (Default|UpdateAmmoNumber _hudref _result (Variables|Default|GetPistol%20Ammo))))
        (bind _outhit (Collision|LineTraceByChannel _returnvalue_2 (+ _returnvalue_2 (* (Transformation|GetActorForwardVector _returnvalue) (Variables|Default|GetLineTraceBullets))) "TraceTypeQuery1" false 0 "None"))
        (bind _asbp_master_range_2 (Utilities|Casting|CastToBP_MasterRange (Variables|Default|GetMain%20Weapon)))
        (Components|Animation|PlayAnimation (Variables|/Game/Blueprints/Weapons/BP_MasterWeapons.BP_MasterWeapons_C|GetWeaponMesh _asbp_master_range_2) (Variables|/Game/Blueprints/Weapons/BP_MasterRange.BP_MasterRange_C|GetAnimToPlay _asbp_master_range_2) false)
        (bind _asbp_skeleton_5 (Utilities|Casting|CastToBP_Skeleton5 (.HitActor (Collision|BreakHitResult _outhit)))
          (:then
            (Game|Damage|ApplyDamage _asbp_skeleton_5 (Variables|/Game/Blueprints/Weapons/BP_MasterWeapons.BP_MasterWeapons_C|GetDamage _asbp_master_range_2) (Game|GetPlayerController 0) (Game|GetPlayerCharacter 0) "/Script/Engine.DamageType")
            (Default|CrossHairHit (Variables|Default|GetHUDRef)))
          (:CastFailed
            _))
        (Effects|SpawnEmitteratLocation "/Game/MilitaryWeapSilver/FX/P_Impact_Metal_Small_01.P_Impact_Metal_Small_01" (.ImpactPoint (Collision|BreakHitResult _outhit)))
        (if (and (Variables|/Game/Blueprints/Weapons/BP_MasterRange.BP_MasterRange_C|GetIsAutomatic? _asbp_master_range_2) (Variables|Default|GetKeepFiring?))
          (Utilities|FlowControl|Delay (Variables|/Game/Blueprints/Weapons/BP_MasterRange.BP_MasterRange_C|GetCoolDownAutoFire _asbp_master_range_2))
          (CallFunction|ContinueFire))))
    (else
      (CallFunction|ManualReload))))

(event Custom|ManualReload
  ;[0.15 0.15 0.15 0.5] Reload
  (if (not (Variables|Default|GetIsReloading?))
    (bind _asbp_master_range (Utilities|Casting|CastToBP_MasterRange (Variables|Default|GetMain%20Weapon)))
    (Variables|Default|SetIsReloading? true)
    (switch Utilities|FlowControl|Switch|SwitchonEnum_WeaponNAME (Variables|/Game/Blueprints/Weapons/BP_MasterWeapons.BP_MasterWeapons_C|GetWeapon%20Name _asbp_master_range)
      (:NewEnumerator3
        (Variables|Default|SetAnimReloadMontage "/Game/RifleAnimationAdventureMan/RifleAdventureManReload_Rifle_Hip_Montage.RifleAdventureManReload_Rifle_Hip_Montage")
        (bind _output_get (Variables|Default|SetAssaultRifleAmmo (+ (Variables|/Game/Blueprints/Weapons/BP_MasterRange.BP_MasterRange_C|GetAmmo _asbp_master_range) (Variables|Default|GetAssaultRifleAmmo))))
        (if (>= _output_get 30)
          (Variables|Default|SetAssaultRifleAmmo (- (Variables|Default|GetAssaultRifleAmmo) (Variables|/Game/Blueprints/Weapons/BP_MasterRange.BP_MasterRange_C|GetMaxAmmo _asbp_master_range)))
          (Variables|/Game/Blueprints/Weapons/BP_MasterRange.BP_MasterRange_C|SetAmmo _asbp_master_range 30)
          (Animation|PlayAnimMontage (Variables|Default|GetAnimReloadMontage) 1.0 "None" :!label _label)
          (elif (>= _output_get 1)
            (Variables|/Game/Blueprints/Weapons/BP_MasterRange.BP_MasterRange_C|SetAmmo _asbp_master_range (Variables|Default|GetAssaultRifleAmmo))
            (Variables|Default|SetAssaultRifleAmmo 0)
            (goto _label))))
      (:NewEnumerator4
        (Variables|Default|SetAnimReloadMontage "/Game/RifleAnimationAdventureMan/RifleAdventureManReload_Pistol_Montage.RifleAdventureManReload_Pistol_Montage")
        (bind _output_get_2 (Variables|Default|SetPistol%20Ammo (+ (Variables|/Game/Blueprints/Weapons/BP_MasterRange.BP_MasterRange_C|GetAmmo _asbp_master_range) (Variables|Default|GetPistol%20Ammo))))
        (if (>= _output_get_2 15)
          (Variables|Default|SetPistol%20Ammo (- (Variables|Default|GetPistol%20Ammo) (Variables|/Game/Blueprints/Weapons/BP_MasterRange.BP_MasterRange_C|GetMaxAmmo _asbp_master_range)))
          (Variables|/Game/Blueprints/Weapons/BP_MasterRange.BP_MasterRange_C|SetAmmo _asbp_master_range 15)
          (goto _label)
          (elif (>= _output_get_2 1)
            (Variables|/Game/Blueprints/Weapons/BP_MasterRange.BP_MasterRange_C|SetAmmo _asbp_master_range (Variables|Default|GetPistol%20Ammo))
            (Variables|Default|SetPistol%20Ammo 0)
            (goto _label)))))))

(event Custom|NearVendingMachine
  (params (VendingMachineNearPlayer :type BP%20Master%20Vending%20Machine%20Object%20Reference) (WeaponName :type String))
  ;[0.15 0.15 0.15 0.5] Vending machines
  (Variables|Default|SetVendingMachineNearPlayer VendingMachineNearPlayer)
  (Default|DisplayPickupInfo (Variables|Default|GetPickupWeaponRef) WeaponName false))

(event Custom|ExitingVendingMachine
  ;[0.15 0.15 0.15 0.5] Vending machines
  (Variables|Default|SetVendingMachineNearPlayer 0)
  (Default|HidePickupInfo (Variables|Default|GetPickupWeaponRef)))

(event Custom|InteractWithVendingMachine
  (bind _vendingmachinenearplayer (Variables|Default|GetVendingMachineNearPlayer))
  (bind _price (Variables|/Game/Blueprints/VendingMachine/BP_MasterVendingMachine.BP_MasterVendingMachine_C|GetPrice _vendingmachinenearplayer))
  ;[0.15 0.15 0.15 0.5] Vending machines
  (if (not (<= (Variables|Default|GetCurrentMoney) _price))
    (switch Utilities|FlowControl|Switch|SwitchonE_VendingMachineType (Variables|/Game/Blueprints/VendingMachine/BP_MasterVendingMachine.BP_MasterVendingMachine_C|GetVendingMachineType _vendingmachinenearplayer)
      (:NewEnumerator0
        (CallFunction|AddHealthtoPlayerVendingMachine))
      (:NewEnumerator1
        (CallFunction|PowerUpVendingMachine))
      (:NewEnumerator2
        (CallFunction|AddAmmotoPlayerVendingMachine)))
    (bind _output_get (Variables|Default|SetCurrentMoney (- (Variables|Default|GetCurrentMoney) _price)))
    (Default|UpdateMoney (Variables|Default|GetHUDRef) _output_get)))

(event Custom|AddHealthToPlayer_VendingMachine
  ;[0.15 0.15 0.15 0.5] Vending machines
  ;;[0.15 0.15 0.15 0.5] Health Vending Machine
  (if (< (Variables|Default|GetHealth) (Variables|Default|GetHealthMax))
    (Variables|Default|SetHealth (Variables|Default|GetHealthMax))
    (Widget|SetVisibility (Variables|/Game/Blueprints/UI/WBP_TakeDamage.WBP_TakeDamage_C|GetIMG_FirstStep (Variables|Default|GetTakeDamageRef)) "Hidden")))

(event Custom|AddAmmoToPlayer_VendingMachine
  ;[0.15 0.15 0.15 0.5] Vending machines
  ;;[0.15 0.15 0.15 0.5] Ammo Vending
  (bind _asbp_master_range (Utilities|Casting|CastToBP_MasterRange (Variables|Default|GetMain%20Weapon)))
  (switch Utilities|FlowControl|Switch|SwitchonEnum_WeaponNAME (Variables|/Game/Blueprints/Weapons/BP_MasterWeapons.BP_MasterWeapons_C|GetWeapon%20Name _asbp_master_range)
    (:NewEnumerator3
      (if (< (Variables|Default|GetAssaultRifleAmmo) (Variables|Default|GetAssault%20Rifle%20Ammo%20Max))
        (bind _output_get (Variables|Default|SetAssaultRifleAmmo (Variables|Default|GetAssault%20Rifle%20Ammo%20Max)))
        (Default|UpdateAmmoNumber (Variables|Default|GetHUDRef) (Variables|/Game/Blueprints/Weapons/BP_MasterRange.BP_MasterRange_C|GetAmmo _asbp_master_range) _output_get)))
    (:NewEnumerator4
      (if (< (Variables|Default|GetPistol%20Ammo) (Variables|Default|GetPistol%20AmmoMax))
        (bind _output_get_2 (Variables|Default|SetPistol%20Ammo (Variables|Default|GetPistol%20AmmoMax)))
        (Default|UpdateAmmoNumber (Variables|Default|GetHUDRef) (Variables|/Game/Blueprints/Weapons/BP_MasterRange.BP_MasterRange_C|GetAmmo _asbp_master_range) _output_get_2)))))

(event Custom|PowerUp_VendingMachine
  ;[0.15 0.15 0.15 0.5] Vending machines
  (bind _asbp_master_range (Utilities|Casting|CastToBP_MasterRange (Variables|Default|GetMain%20Weapon)))
  (switch Utilities|FlowControl|Switch|SwitchonEnum_WeaponNAME (Variables|/Game/Blueprints/Weapons/BP_MasterWeapons.BP_MasterWeapons_C|GetWeapon%20Name _asbp_master_range)
    (:NewEnumerator3
      (Variables|/Game/Blueprints/Weapons/BP_MasterWeapons.BP_MasterWeapons_C|SetDamage _asbp_master_range (* (Variables|/Game/Blueprints/Weapons/BP_MasterWeapons.BP_MasterWeapons_C|GetDamage _asbp_master_range) 2.0))
      (Variables|Default|SetAssault%20Rifle%20Ammo%20Max (* (Variables|Default|GetAssault%20Rifle%20Ammo%20Max) 3)))))

(event Input|EnhancedActionEvents|EnhancedInputActionIA_AdventureMovement
  (params (ActionValue :type Vector%202D%20Structure) (ElapsedSeconds :type Float%20%28double-precision%29) (TriggeredSeconds :type Float%20%28double-precision%29) (InputAction :type Input%20Action%20Object%20Reference :default "/Game/Blueprints/Inputs/Actions/IA_AdventureMovement.IA_AdventureMovement"))
  (bind _returnvalue (Pawn|GetControlRotation :!class /Script/Engine.Pawn))
  (bind _hudref (Variables|Default|GetHUDRef))
  ;[0.15 0.15 0.15 0.5] Mouvement
  (Pawn|Input|AddMovementInput (Math|Vector|GetRightVector (Math|Rotator|MakeRotator 0.0 0.0 (.yaw _returnvalue))) (.x ActionValue) false)
  (Pawn|Input|AddMovementInput (Math|Vector|GetForwardVector (Math|Rotator|MakeRotator 0.0 0.0 (.yaw _returnvalue))) (.y ActionValue) false)
  (if (or (!= (.x ActionValue) 0.0) (!= (.y ActionValue) 0.0))
    (UserInterface|Animation|PlayAnimation _hudref (Variables|/Game/Blueprints/UI/WBP_HUD.WBP_HUD_C|GetAimingExpand _hudref) 0.0 1 "Reverse" 1.0 false)))

(event Input|EnhancedActionEvents|EnhancedInputActionIA_AdventureJump
  (params (ActionValue :type Boolean) (ElapsedSeconds :type Float%20%28double-precision%29) (TriggeredSeconds :type Float%20%28double-precision%29) (InputAction :type Input%20Action%20Object%20Reference :default "/Game/Blueprints/Inputs/Actions/IA_AdventureJump.IA_AdventureJump"))
  ;[0.15 0.15 0.15 0.5] Mouvement
  (:Started
    (Character|Jump))
  (:Completed
    (Character|StopJumping)))

(event Input|EnhancedActionEvents|EnhancedInputActionIA_AdventureCamera
  (params (ActionValue :type Vector%202D%20Structure) (ElapsedSeconds :type Float%20%28double-precision%29) (TriggeredSeconds :type Float%20%28double-precision%29) (InputAction :type Input%20Action%20Object%20Reference :default "/Game/Blueprints/Inputs/Actions/IA_AdventureCamera.IA_AdventureCamera"))
  ;[0.15 0.15 0.15 0.5] Mouvement
  (Pawn|Input|AddControllerYawInput (.x ActionValue))
  (Pawn|Input|AddControllerPitchInput (.y ActionValue)))

(event Input|EnhancedActionEvents|EnhancedInputActionIA_AdventurePickup
  (params (ActionValue :type Boolean) (ElapsedSeconds :type Float%20%28double-precision%29) (TriggeredSeconds :type Float%20%28double-precision%29) (InputAction :type Input%20Action%20Object%20Reference :default "/Game/Blueprints/Inputs/Actions/IA_AdventurePickup.IA_AdventurePickup"))
  (bind _obstacles (Variables|Default|GetObstacles))
  (bind _hudref (Variables|Default|GetHUDRef))
  (bind _price (Variables|/Game/Maps/Blueprints/BP_MasterObstacles.BP_MasterObstacles_C|GetPrice _obstacles))
  (bind _txt_ammo (Variables|/Game/Blueprints/UI/WBP_HUD.WBP_HUD_C|GetTXT_Ammo _hudref))
  ;[0.15 0.15 0.15 0.5] PickUp
  (:Started
    (Utilities|IsValid (Variables|Default|GetPickUpWeapon)
      (:Is%20Valid
        (Utilities|IsValid (Variables|Default|GetMain%20Weapon)
          (:Is%20Valid
            (bind _output_get (Variables|Default|SetSecondaryWeapon (Variables|Default|GetPickUpWeapon)))
            (if (Variables|/Game/Blueprints/Weapons/BP_MasterWeapons.BP_MasterWeapons_C|GetMelee%20Weapon? _output_get)
              (Variables|Default|SetSocketToAttachWeapon "KatanaWeaponBack")
              (else
                (Variables|Default|SetSocketToAttachWeapon "ARWeaponBack")))
            (Transformation|AttachComponentToComponent (Variables|Default|GetSecondaryWeapon) (Variables|Character|GetMesh) (Variables|Default|GetSocketToAttachWeapon) "SnapToTarget" "SnapToTarget" "KeepRelative" true)
            (Variables|/Script/Engine.RotatingMovementComponent|SetRotationRate (Variables|/Game/Blueprints/Weapons/BP_MasterWeapons.BP_MasterWeapons_C|GetRotatingMovement (Variables|Default|GetSecondaryWeapon)) "0, 0, 0")
            (Transformation|SetRelativeRotation (Variables|/Game/Blueprints/Weapons/BP_MasterWeapons.BP_MasterWeapons_C|GetWeaponMesh (Variables|Default|GetSecondaryWeapon)) "0, 0, 0" false false)
            (Transformation|SetRelativeLocation (Variables|/Game/Blueprints/Weapons/BP_MasterWeapons.BP_MasterWeapons_C|GetWeaponMesh (Variables|Default|GetSecondaryWeapon)) "0, 0, 0" false true)
            (Variables|/Game/Blueprints/Weapons/BP_MasterWeapons.BP_MasterWeapons_C|SetIsEquipped? (Variables|Default|GetSecondaryWeapon) true)
            (Variables|Default|SetPickUpWeapon 0)
            (Default|HidePickupInfo (Variables|Default|GetPickupWeaponRef)))
          (:Is%20Not%20Valid
            (bind _output_get_2 (Variables|Default|SetMain%20Weapon (Variables|Default|GetPickUpWeapon)))
            (if (Variables|/Game/Blueprints/Weapons/BP_MasterWeapons.BP_MasterWeapons_C|GetMelee%20Weapon? _output_get_2)
              (Variables|Default|SetHasWeapon true)
              (Variables|Default|SetRifleEquipped false)
              (Variables|Default|SetKatanaEquipped? true)
              (Variables|Default|SetSocketToAttachWeapon "KatanaRightHand")
              (else
                (Variables|Default|SetHasWeapon true)
                (Variables|Default|SetRifleEquipped true)
                (Variables|Default|SetKatanaEquipped? false)
                (Variables|Default|SetSocketToAttachWeapon "RifleRightHand")
                (Variables|/Script/UMG.Widget|SetVisibility (Variables|/Game/Blueprints/UI/WBP_HUD.WBP_HUD_C|GetIMG_Crosshair (Variables|Default|GetHUDRef)) "Visible")))
            (Transformation|AttachComponentToComponent (Variables|Default|GetMain%20Weapon) (Variables|Character|GetMesh) (Variables|Default|GetSocketToAttachWeapon) "SnapToTarget" "SnapToTarget" "KeepRelative" true)
            (Variables|/Script/Engine.RotatingMovementComponent|SetRotationRate (Variables|/Game/Blueprints/Weapons/BP_MasterWeapons.BP_MasterWeapons_C|GetRotatingMovement (Variables|Default|GetMain%20Weapon)) "0, 0, 0")
            (Transformation|SetRelativeLocationAndRotation (Variables|/Game/Blueprints/Weapons/BP_MasterWeapons.BP_MasterWeapons_C|GetWeaponMesh (Variables|Default|GetMain%20Weapon)) "0, 0, 0" "0, 0, 0" false true)
            (Variables|/Game/Blueprints/Weapons/BP_MasterWeapons.BP_MasterWeapons_C|SetIsEquipped? (Variables|Default|GetPickUpWeapon) true)
            (Variables|Default|SetPickUpWeapon 0)
            (Default|HidePickupInfo (Variables|Default|GetPickupWeaponRef))
            (if (Variables|/Game/Blueprints/Weapons/BP_MasterWeapons.BP_MasterWeapons_C|GetMelee%20Weapon? (Variables|Default|GetMain%20Weapon))
              (Variables|Default|SetWeaponImage "/Game/Blueprints/UI/HIT/V2_Banner_Katana.V2_Banner_Katana")
              (Variables|/Script/UMG.Widget|SetVisibility _txt_ammo "Hidden")
              (else
                (Variables|Default|SetWeaponImage "/Game/Blueprints/UI/HIT/V2_Banner_AR.V2_Banner_AR")
                (Variables|/Script/UMG.Widget|SetVisibility _txt_ammo "Visible")))
            (Default|ChangeWeaponName _hudref (Utilities|String|EnumtoString (Variables|/Game/Blueprints/Weapons/BP_MasterWeapons.BP_MasterWeapons_C|GetWeapon%20Name (Variables|Default|GetMain%20Weapon))) (Variables|Default|GetWeaponImage))
            (bind _asbp_master_range (Utilities|Casting|CastToBP_MasterRange (Variables|Default|GetMain%20Weapon)))
            (Default|UpdateAmmoNumber _hudref (Variables|/Game/Blueprints/Weapons/BP_MasterRange.BP_MasterRange_C|GetAmmo _asbp_master_range) (Variables|/Game/Blueprints/Weapons/BP_MasterRange.BP_MasterRange_C|GetMaxAmmo _asbp_master_range)))))
      (:Is%20Not%20Valid
        (Utilities|IsValid (Variables|Default|GetVendingMachineNearPlayer)
          (:Is%20Valid
            (CallFunction|InteractwithVendingMachine))
          (:Is%20Not%20Valid
            (Utilities|IsValid _obstacles
              (:Is%20Valid
                (if (>= (Variables|Default|GetCurrentMoney) _price)
                  (bind _output_get_3 (Variables|Default|SetCurrentMoney (- (Variables|Default|GetCurrentMoney) _price)))
                  (Default|OpenObstacles _obstacles)
                  (Default|UpdateMoney (Variables|Default|GetHUDRef) _output_get_3))))))))))

(event Input|EnhancedActionEvents|EnhancedInputActionIA_AdventureFire
  (params (ActionValue :type Boolean) (ElapsedSeconds :type Float%20%28double-precision%29) (TriggeredSeconds :type Float%20%28double-precision%29) (InputAction :type Input%20Action%20Object%20Reference :default "/Game/Blueprints/Inputs/Actions/IA_AdventureFire.IA_AdventureFire"))
  (bind _returnvalue (Game|GetPlayerCameraManager 0))
  (bind _hudref (Variables|Default|GetHUDRef))
  (bind _returnvalue_2 (Camera|GetCameraLocation _returnvalue))
  ;[0.15 0.15 0.15 0.5] Attack
  (:Started
    (if (Variables|Default|GetHasWeapon)
      (if (and (Variables|Default|GetRifleEquipped) (not (Variables|Default|GetIsReloading?)))
        ;;[0.15 0.15 0.15 0.5] RifleAttack
        (Variables|Default|SetKeepFiring? true)
        (bind _asbp_master_range (Utilities|Casting|CastToBP_MasterRange (Variables|Default|GetMain%20Weapon)))
        (if (> (Variables|/Game/Blueprints/Weapons/BP_MasterRange.BP_MasterRange_C|GetAmmo _asbp_master_range) 0)
          (bind _result (Math|Integer|DecrementInt (Variables|/Game/Blueprints/Weapons/BP_MasterRange.BP_MasterRange_C|GetAmmo _asbp_master_range))
            (:%20%20
              (switch Utilities|FlowControl|Switch|SwitchonEnum_WeaponNAME (Variables|/Game/Blueprints/Weapons/BP_MasterWeapons.BP_MasterWeapons_C|GetWeapon%20Name _asbp_master_range)
                (:NewEnumerator3
                  (Default|UpdateAmmoNumber _hudref _result (Variables|Default|GetAssaultRifleAmmo)))
                (:NewEnumerator4
                  (Default|UpdateAmmoNumber _hudref _result (Variables|Default|GetPistol%20Ammo))))
              (bind _outhit (Collision|LineTraceByChannel _returnvalue_2 (+ _returnvalue_2 (* (Transformation|GetActorForwardVector _returnvalue) (Variables|Default|GetLineTraceBullets))) "TraceTypeQuery1" false 0 "None"))
              (bind _asbp_master_range_2 (Utilities|Casting|CastToBP_MasterRange (Variables|Default|GetMain%20Weapon)))
              (Components|Animation|PlayAnimation (Variables|/Game/Blueprints/Weapons/BP_MasterWeapons.BP_MasterWeapons_C|GetWeaponMesh _asbp_master_range_2) (Variables|/Game/Blueprints/Weapons/BP_MasterRange.BP_MasterRange_C|GetAnimToPlay _asbp_master_range_2) false)
              (bind _asbp_skeleton_5 (Utilities|Casting|CastToBP_Skeleton5 (.HitActor (Collision|BreakHitResult _outhit)))
                (:then
                  (Game|Damage|ApplyDamage _asbp_skeleton_5 (Variables|/Game/Blueprints/Weapons/BP_MasterWeapons.BP_MasterWeapons_C|GetDamage _asbp_master_range_2) (Game|GetPlayerController 0) (Game|GetPlayerCharacter 0) "/Script/Engine.DamageType")
                  (Default|CrossHairHit (Variables|Default|GetHUDRef)))
                (:CastFailed
                  _))
              (Effects|SpawnEmitteratLocation "/Game/MilitaryWeapSilver/FX/P_Impact_Metal_Small_01.P_Impact_Metal_Small_01" (.ImpactPoint (Collision|BreakHitResult _outhit)))
              (if (and (Variables|/Game/Blueprints/Weapons/BP_MasterRange.BP_MasterRange_C|GetIsAutomatic? _asbp_master_range_2) (Variables|Default|GetKeepFiring?))
                (Utilities|FlowControl|Delay (Variables|/Game/Blueprints/Weapons/BP_MasterRange.BP_MasterRange_C|GetCoolDownAutoFire _asbp_master_range_2))
                (CallFunction|ContinueFire))))
          (else
            (CallFunction|ManualReload)))
        (else
          ;;[0.15 0.15 0.15 0.5] Katana attack
          (if (and (Variables|Default|GetKatanaEquipped?) (not (Variables|Default|GetIsAttacking?)))
            (Utilities|Casting|CastToBP_MasterMelee (Variables|Default|GetMain%20Weapon))
            (switch int (Variables|Default|GetComboIndex)
              (:0
                (Variables|Default|SetSectionAttackMontage "FirstAttack"))
              (:1
                (Variables|Default|SetSectionAttackMontage "SecondAttack"))
              (:2
                (Variables|Default|SetSectionAttackMontage "ThirdAttack")))
            (Animation|PlayAnimMontage "/Game/Retarget_KatanaAdventureMan/AM_KatanaAttack.AM_KatanaAttack" 1.0 (Variables|Default|GetSectionAttackMontage))
            (Variables|Default|SetIsAttacking? true))))))
  (:Completed
    (Variables|Default|SetKeepFiring? false)))

(event Input|EnhancedActionEvents|EnhancedInputActionIA_AdventurePause
  (params (ActionValue :type Boolean) (ElapsedSeconds :type Float%20%28double-precision%29) (TriggeredSeconds :type Float%20%28double-precision%29) (InputAction :type Input%20Action%20Object%20Reference :default "/Game/Blueprints/Inputs/Actions/IA_AdventurePause.IA_AdventurePause"))
  (bind _returnvalue (Game|GetPlayerController 0))
  ;[0.15 0.15 0.15 0.5] Pause
  (:Started
    (Game|SetGamePaused true)
    (bind _returnvalue_2 (UserInterface|CreateWidget "/Game/Blueprints/UI/PauseScreen/WBP_Pause.WBP_Pause_C"))
    (UserInterface|Viewport|AddtoViewport _returnvalue_2 0)
    (Variables|/Script/Engine.PlayerController|SetbShowMouseCursor _returnvalue true)
    (Input|SetInputModeUIOnly _returnvalue _returnvalue_2 "DoNotLock" false)))

(event Input|EnhancedActionEvents|EnhancedInputActionIA_Aim
  (params (ActionValue :type Boolean) (ElapsedSeconds :type Float%20%28double-precision%29) (TriggeredSeconds :type Float%20%28double-precision%29) (InputAction :type Input%20Action%20Object%20Reference :default "/Game/Blueprints/Inputs/Actions/IA_Aim.IA_Aim"))
  (bind _hudref (Variables|Default|GetHUDRef))
  (bind _hudref_2 (Variables|Default|GetHUDRef))
  ;[0.15 0.15 0.15 0.5] Aim
  (:Started
    (if (and (Variables|Default|GetHasWeapon) (Variables|Default|GetRifleEquipped))
      (if (not (Variables|Default|GetIsAiming?))
        (Variables|Default|SetIsAiming? true)
        (UserInterface|Animation|PlayAnimation _hudref_2 (Variables|/Game/Blueprints/UI/WBP_HUD.WBP_HUD_C|GetAimingShrink _hudref_2) 0.0 1 "Forward" 1.0 false)
        (Variables|/Script/Engine.CharacterMovementComponent|SetMaxWalkSpeed (Variables|Character|GetCharacterMovement) 3e+02)
        (bind _zoom (Timeline|ZoomAim PlayFromStart)
          (:Update
            (Camera|SetFieldOfView (Variables|Default|GetCamera) _zoom))))))
  (:Completed
    (if (and (Variables|Default|GetHasWeapon) (Variables|Default|GetRifleEquipped))
      (Variables|Default|SetIsAiming? false)
      (UserInterface|Animation|PlayAnimation _hudref (Variables|/Game/Blueprints/UI/WBP_HUD.WBP_HUD_C|GetAimingShrink _hudref) 0.0 1 "Reverse" 1.0 false)
      (Variables|/Script/Engine.CharacterMovementComponent|SetMaxWalkSpeed (Variables|Character|GetCharacterMovement) 6e+02)
      (Timeline|ZoomAim ReverseFromEnd))))

(event Input|EnhancedActionEvents|EnhancedInputActionIA_Reload
  (params (ActionValue :type Boolean) (ElapsedSeconds :type Float%20%28double-precision%29) (TriggeredSeconds :type Float%20%28double-precision%29) (InputAction :type Input%20Action%20Object%20Reference :default "/Game/Blueprints/Inputs/Actions/IA_Reload.IA_Reload"))
  ;[0.15 0.15 0.15 0.5] Reload
  (:Started
    (if (not (Variables|Default|GetIsReloading?))
      (bind _asbp_master_range (Utilities|Casting|CastToBP_MasterRange (Variables|Default|GetMain%20Weapon)))
      (Variables|Default|SetIsReloading? true)
      (switch Utilities|FlowControl|Switch|SwitchonEnum_WeaponNAME (Variables|/Game/Blueprints/Weapons/BP_MasterWeapons.BP_MasterWeapons_C|GetWeapon%20Name _asbp_master_range)
        (:NewEnumerator3
          (Variables|Default|SetAnimReloadMontage "/Game/RifleAnimationAdventureMan/RifleAdventureManReload_Rifle_Hip_Montage.RifleAdventureManReload_Rifle_Hip_Montage")
          (bind _output_get (Variables|Default|SetAssaultRifleAmmo (+ (Variables|/Game/Blueprints/Weapons/BP_MasterRange.BP_MasterRange_C|GetAmmo _asbp_master_range) (Variables|Default|GetAssaultRifleAmmo))))
          (if (>= _output_get 30)
            (Variables|Default|SetAssaultRifleAmmo (- (Variables|Default|GetAssaultRifleAmmo) (Variables|/Game/Blueprints/Weapons/BP_MasterRange.BP_MasterRange_C|GetMaxAmmo _asbp_master_range)))
            (Variables|/Game/Blueprints/Weapons/BP_MasterRange.BP_MasterRange_C|SetAmmo _asbp_master_range 30)
            (Animation|PlayAnimMontage (Variables|Default|GetAnimReloadMontage) 1.0 "None" :!label _label)
            (elif (>= _output_get 1)
              (Variables|/Game/Blueprints/Weapons/BP_MasterRange.BP_MasterRange_C|SetAmmo _asbp_master_range (Variables|Default|GetAssaultRifleAmmo))
              (Variables|Default|SetAssaultRifleAmmo 0)
              (goto _label))))
        (:NewEnumerator4
          (Variables|Default|SetAnimReloadMontage "/Game/RifleAnimationAdventureMan/RifleAdventureManReload_Pistol_Montage.RifleAdventureManReload_Pistol_Montage")
          (bind _output_get_2 (Variables|Default|SetPistol%20Ammo (+ (Variables|/Game/Blueprints/Weapons/BP_MasterRange.BP_MasterRange_C|GetAmmo _asbp_master_range) (Variables|Default|GetPistol%20Ammo))))
          (if (>= _output_get_2 15)
            (Variables|Default|SetPistol%20Ammo (- (Variables|Default|GetPistol%20Ammo) (Variables|/Game/Blueprints/Weapons/BP_MasterRange.BP_MasterRange_C|GetMaxAmmo _asbp_master_range)))
            (Variables|/Game/Blueprints/Weapons/BP_MasterRange.BP_MasterRange_C|SetAmmo _asbp_master_range 15)
            (goto _label)
            (elif (>= _output_get_2 1)
              (Variables|/Game/Blueprints/Weapons/BP_MasterRange.BP_MasterRange_C|SetAmmo _asbp_master_range (Variables|Default|GetPistol%20Ammo))
              (Variables|Default|SetPistol%20Ammo 0)
              (goto _label))))))))

(event Input|EnhancedActionEvents|EnhancedInputActionIA_AdventureSwitchWeapon
  (params (ActionValue :type Boolean) (ElapsedSeconds :type Float%20%28double-precision%29) (TriggeredSeconds :type Float%20%28double-precision%29) (InputAction :type Input%20Action%20Object%20Reference :default "/Game/Blueprints/Inputs/Actions/IA_AdventureSwitchWeapon.IA_AdventureSwitchWeapon"))
  (bind _hudref (Variables|Default|GetHUDRef))
  (bind _txt_ammo (Variables|/Game/Blueprints/UI/WBP_HUD.WBP_HUD_C|GetTXT_Ammo _hudref))
  ;[0.15 0.15 0.15 0.5] Switch Weapon
  (:Started
    (Utilities|IsValid (Variables|Default|GetMain%20Weapon)
      (:Is%20Valid
        (Utilities|IsValid (Variables|Default|GetSecondaryWeapon)
          (:Is%20Valid
            (Variables|Default|SetTempSwitchingWeapon (Variables|Default|GetSecondaryWeapon))
            (if (Variables|/Game/Blueprints/Weapons/BP_MasterWeapons.BP_MasterWeapons_C|GetMelee%20Weapon? (Variables|Default|GetMain%20Weapon))
              (Variables|Default|SetHasWeapon true)
              (Variables|Default|SetRifleEquipped true)
              (Variables|Default|SetKatanaEquipped? false)
              (Variables|Default|SetSocketToAttachWeapon "RifleRightHand")
              (Variables|/Script/UMG.Widget|SetVisibility (Variables|/Game/Blueprints/UI/WBP_HUD.WBP_HUD_C|GetIMG_Crosshair (Variables|Default|GetHUDRef)) "Visible")
              (Variables|Default|SetEquipAnim "/Game/RifleAnimationAdventureMan/AM_EquipRiffle.AM_EquipRiffle")
              (Variables|Default|SetEquipAnimDelay 1.5)
              (else
                (Variables|Default|SetHasWeapon true)
                (Variables|Default|SetRifleEquipped false)
                (Variables|Default|SetKatanaEquipped? true)
                (Variables|Default|SetSocketToAttachWeapon "KatanaRightHand")
                (Variables|Default|SetEquipAnim "/Game/Retarget_KatanaAdventureMan/AM_EquipKatana.AM_EquipKatana")
                (Variables|Default|SetEquipAnimDelay 0.5)))
            (Animation|PlayAnimMontage (Variables|Default|GetEquipAnim) 1.0 "None")
            (Utilities|FlowControl|Delay (Variables|Default|GetEquipAnimDelay))
            (Transformation|AttachComponentToComponent (Variables|Default|GetSecondaryWeapon) (Variables|Character|GetMesh) (Variables|Default|GetSocketToAttachWeapon) "SnapToTarget" "SnapToTarget" "KeepRelative" true)
            (if (Variables|/Game/Blueprints/Weapons/BP_MasterWeapons.BP_MasterWeapons_C|GetMelee%20Weapon? (Variables|Default|GetSecondaryWeapon))
              (Variables|Default|SetSocketToAttachWeapon "ARWeaponBack")
              (else
                (Variables|Default|SetSocketToAttachWeapon "KatanaWeaponBack")))
            (Transformation|AttachComponentToComponent (Variables|Default|GetMain%20Weapon) (Variables|Character|GetMesh) (Variables|Default|GetSocketToAttachWeapon) "SnapToTarget" "SnapToTarget" "KeepRelative" true)
            (Transformation|SetRelativeLocationAndRotation (Variables|/Game/Blueprints/Weapons/BP_MasterWeapons.BP_MasterWeapons_C|GetWeaponMesh (Variables|Default|GetMain%20Weapon)) "0, 0, 0" "0, 0, 0" false true)
            (Variables|Default|SetSecondaryWeapon (Variables|Default|GetMain%20Weapon))
            (Variables|Default|SetMain%20Weapon (Variables|Default|GetTempSwitchingWeapon))
            (Variables|Default|SetTempSwitchingWeapon 0)
            (if (Variables|/Game/Blueprints/Weapons/BP_MasterWeapons.BP_MasterWeapons_C|GetMelee%20Weapon? (Variables|Default|GetMain%20Weapon))
              (Variables|Default|SetWeaponImage "/Game/Blueprints/UI/HIT/V2_Banner_Katana.V2_Banner_Katana")
              (Variables|/Script/UMG.Widget|SetVisibility _txt_ammo "Hidden")
              (else
                (Variables|Default|SetWeaponImage "/Game/Blueprints/UI/HIT/V2_Banner_AR.V2_Banner_AR")
                (Variables|/Script/UMG.Widget|SetVisibility _txt_ammo "Visible")))
            (Default|ChangeWeaponName (Variables|Default|GetHUDRef) (Utilities|String|EnumtoString (Variables|/Game/Blueprints/Weapons/BP_MasterWeapons.BP_MasterWeapons_C|GetWeapon%20Name (Variables|Default|GetMain%20Weapon))) (Variables|Default|GetWeaponImage))))))))

(event EventBeginPlay
  (bind _returnvalue (Game|GetPlayerController 0))
  ;[0.15 0.15 0.15 0.5] Begin Play
  (Utilities|IsValid _returnvalue
    (:Is%20Valid
      (Input|AddMappingContext (PlayerController|LocalPlayerSubsystems|GetEnhancedInputLocalPlayerSubsystem _returnvalue) "/Game/Blueprints/Inputs/IMC_AdventureMan.IMC_AdventureMan" 0 "(bIgnoreAllPressedKeysUntilRelease=True,bForceImmediately=False,bNotifyUserSettings=False)")
      (bind _returnvalue_2 (UserInterface|CreateWidget "/Game/Blueprints/UI/WBP_PickUpWeapon.WBP_PickUpWeapon_C"))
      (bind _output_get (Variables|Default|SetPickupWeaponRef _returnvalue_2))
      (UserInterface|Viewport|AddtoViewport _output_get 0)
      (Default|HidePickupInfo (Variables|Default|GetPickupWeaponRef))
      (bind _returnvalue_3 (UserInterface|CreateWidget "/Game/Blueprints/UI/WBP_HUD.WBP_HUD_C"))
      (bind _output_get_2 (Variables|Default|SetHUDRef _returnvalue_3))
      (UserInterface|Viewport|AddtoViewport _output_get_2 0)
      (bind _returnvalue_4 (UserInterface|CreateWidget "/Game/Blueprints/UI/WBP_TakeDamage.WBP_TakeDamage_C"))
      (bind _output_get_3 (Variables|Default|SetTakeDamageRef _returnvalue_4))
      (UserInterface|Viewport|AddtoViewport _output_get_3 0))))

(fn ConstructionScript)