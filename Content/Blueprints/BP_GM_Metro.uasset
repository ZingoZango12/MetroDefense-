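; BP_GM_Metro, apparently the Metro game mode, runs an endless enemy wave loop.
; After a startup delay it shows the wave number on the player's HUD, plays a sound and tells BP_AISpwaner to spawn the wave.
; SkeletonDeath decrements the alive count and ends the wave once it drops below zero.
; EndOfWave plays a jingle, grows the next wave's size with the wave number and re-announces after a pause.
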(event Custom|Announce%20Wave
  (bind _player_refrence (Variables|Default|GetPlayer%20Refrence))
  (bind _hudref (Variables|/Game/Blueprints/Player/BP_AdventureMan.BP_AdventureMan_C|GetHUDRef _player_refrence))
  ;[0.15 0.15 0.15 0.5] Update Wave hud Number/ SFX / make number glow
  (Utilities|IsValid _player_refrence
    (:Is%20Valid
      (Utilities|IsValid _hudref
        (:Is%20Valid
          (Default|ChangeWaveNumber _hudref (Variables|Default|GetCurrent%20Wave))
          (Audio|PlaySound2D "/Game/Sound/tmpq7xew6z6.tmpq7xew6z6" 1.0 1.0 0.0 0 0)
          (CallFunction|SpawnNextWave))))))

(event Custom|Spawn%20Next%20Wave
  (bind _returnvalue (Actor|GetActorOfClass "/Game/Blueprints/AIspawn/BP_AISpwaner.BP_AISpwaner_C"))
  (Utilities|IsValid _returnvalue
    (:Is%20Valid
      (Default|SpawnWave _returnvalue (Variables|Default|GetEntityToSpawn)))))

(event Custom|EndOfWave
  (Audio|PlaySound2D "/Game/Sound/Jingle_RATP_Metro_2.Jingle_RATP_Metro_2" 1.0 1.0 0.0 0 0)
  (Math|Integer|IncrementInt (Variables|Default|GetCurrent%20Wave)
    (:%20%20
      (bind _output_get (Variables|Default|SetEntityToSpawn (Math|Float|Round (+ (* 1.3 (+ (Variables|Default|GetCurrent%20Wave) 1.0)) (Variables|Default|GetEntityToSpawn)))))
      (Variables|Default|SetCurrent%20Alive%20Entities _output_get)
      (Utilities|FlowControl|Delay 5.0)
      (CallFunction|AnnounceWave))))

(event Custom|Skeleton%20Death
  (bind _output_get (Variables|Default|SetCurrent%20Alive%20Entities (- (Variables|Default|GetCurrent%20Alive%20Entities) 1)))
  (if (< _output_get 0)
    (CallFunction|EndOfWave))
  (Development|PrintString (Utilities|String|ToString(Text) (Utilities|Text|FormatText "Enemies left: {E}" (Variables|Default|GetCurrent%20Alive%20Entities)))))

(event EventBeginPlay
  (bind _asbp_adventure_man (Utilities|Casting|CastToBP_AdventureMan (Game|GetPlayerCharacter 0)))
  (Variables|Default|SetPlayer%20Refrence _asbp_adventure_man)
  (Utilities|FlowControl|Delay 5.0)
  (CallFunction|AnnounceWave))

(fn ConstructionScript)